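; Game logic Blueprint that trains BP_Boxer agents through timed matches and evolutionary selection.
; A Delay on Tick paces 20-second rounds, each ending the previous match and spawning two facing boxers while the agent ID is below 40.
; The first boxer loads the current agent's weights and the second always loads agent 0's.
; EndMatch saves weights and overlap-plus-hit scores; at 40, NaturalSelection runs with mortality and mutation parameters.
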(event EventTick
  (params (DeltaSeconds :type Float%20%28single-precision%29))
  ;[1 1 1] batch
  ;;[1 1 1] match
  (Utilities|FlowControl|Delay 2e+01)
  (bind _returnvalue (Class|GameLogic|GetAgentId))
  (if (< _returnvalue 40)
    (if (Variables|Default|Getfirst_time?)
      (Variables|Default|Setfirst_time? false)
      (else
        (CallFunction|EndMatch)))
    (CallFunction|StartMatch)
    (else
      (Class|GameLogic|NaturalSelection 0.5 0.01 0.01))))

(fn ConstructionScript)

(fn StartMatch
  (bind _returnvalue (Game|SpawnActorfromClass "/Game/Blueprints/BP_Boxer.BP_Boxer_C" (Math|Transform|MakeTransform "-400.000000,-400.000000,39.000000" "0.000000,-45.000000,0.000000") "Undefined" 0 0))
  (bind _output_get (Variables|Default|SetBP_Boxer _returnvalue))
  (bind _returnvalue_2 (Class|GameLogic|GetAgentId))
  (Class|Boxer|LoadWeights _output_get _returnvalue_2)
  (bind _returnvalue_3 (Class|GameLogic|GetAgentId))
  (Class|GameLogic|SetAgentId (+ _returnvalue_3 1))
  (bind _returnvalue_4 (Game|SpawnActorfromClass "/Game/Blueprints/BP_Boxer.BP_Boxer_C" (Math|Transform|MakeTransform "400.000000,400.000000,39.000000" "0.000000,135.000000,0.000000") "Undefined" 0 0))
  (bind _output_get_2 (Variables|Default|SetBP_Boxer2 _returnvalue_4))
  (Class|Boxer|LoadWeights _output_get_2)
  (bind _returnvalue_5 (Class|GameLogic|GetAgentId))
  (Class|GameLogic|SetAgentId (+ _returnvalue_5 1)))

(fn EndMatch
  (bind _bp_boxer2 (Variables|Default|GetBP_Boxer2))
  (bind _bp_boxer (Variables|Default|GetBP_Boxer))
  (bind _returnvalue (Class|GameLogic|GetAgentId))
  (Class|GameLogic|SetAgentId (- _returnvalue 2))
  (bind _returnvalue_2 (Class|GameLogic|GetAgentId))
  (Class|Boxer|SaveWeights (Variables|Default|GetBP_Boxer) _returnvalue_2)
  (Class|GameLogic|SaveScore (+ (Variables|/Game/Blueprints/BP_Boxer.BP_Boxer_C|GetOverlapScore _bp_boxer) (Variables|/Game/Blueprints/BP_Boxer.BP_Boxer_C|GetHitScore _bp_boxer)))
  (Actor|DestroyActor (Variables|Default|GetBP_Boxer))
  (bind _returnvalue_3 (Class|GameLogic|GetAgentId))
  (Class|GameLogic|SetAgentId (+ _returnvalue_3 1))
  (bind _returnvalue_4 (Class|GameLogic|GetAgentId))
  (Class|Boxer|SaveWeights (Variables|Default|GetBP_Boxer2) _returnvalue_4)
  (Class|GameLogic|SaveScore (+ (Variables|/Game/Blueprints/BP_Boxer.BP_Boxer_C|GetOverlapScore _bp_boxer2) (Variables|/Game/Blueprints/BP_Boxer.BP_Boxer_C|GetHitScore _bp_boxer2)))
  (Actor|DestroyActor (Variables|Default|GetBP_Boxer2))
  (bind _returnvalue_5 (Class|GameLogic|GetAgentId))
  (Class|GameLogic|SetAgentId (+ _returnvalue_5 1)))