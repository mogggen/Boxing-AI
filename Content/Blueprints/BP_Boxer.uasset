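; BP_Boxer is a physics-driven boxer controlled by a neural network and scored against an opposing boxer.
; Each tick feeds tagged body-part positions and velocities to the network, substituting opponent head and torso for two slots, then applies its forces to the parts.
; Hits update HitScore by region, with glove and foot formulas, but only when not striking the opponent.
; A fixed overlap box rewards head height through OverlapScore.
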(event EventTick
  (params (DeltaSeconds :type Float%20%28single-precision%29))
  (CallFunction|GetPhysicsInputs)
  (CallFunction|ApplyNeuralNetworkOutputs)
  (CallFunction|RewardProperStance)
  (Development|PrintString (Utilities|String|Append "Hit Score:" (Utilities|String|ToString(Float) (Variables|Default|GetHitScore)) ", Overlap Score: " (Utilities|String|ToString(Float) (Variables|Default|GetOverlapScore)))))

(event Collision|EventHit
  (params (MyComp :type Primitive%20Component%20Object%20Reference) (Other :type Actor%20Object%20Reference) (OtherComp :type Primitive%20Component%20Object%20Reference) (bSelfMoved :type Boolean) (HitLocation :type Vector :default "0, 0, 0") (HitNormal :type Vector :default "0, 0, 0") (NormalImpulse :type Vector :default "0, 0, 0") (Hit :type Hit%20Result%20Structure%20%28by%20ref%29))
  ;[1 1 1] Rewards
  (Variables|Default|SethasStruckOpponent (and (!= (Components|GetOwner OtherComp) self) (== (Utilities|Array|Length (Variables|/Script/Engine.ActorComponent|GetComponentTags OtherComp)) 1)))
  (for _array_element (Variables|/Script/Engine.ActorComponent|GetComponentTags MyComp)
    (bind _index (Utilities|FlowControl|ForLoopwithBreak 0 18)
      (:LoopBody
        (if (Utilities|Name|Equal(Name) _array_element (Utilities|String|StringToName (Utilities|String|ToString(Integer) _index)))
          (switch int _index
            (:0
              (CallFunction|GetHitPenalty (Variables|Default|GetHeadHitPenalty)))
            (:1
              (CallFunction|GetHitPenalty (Variables|Default|GetShoulderHitPenalty) :!label _label))
            (:2
              (CallFunction|GetHitPenalty (Variables|Default|GetTorsoHitPenalty) :!label _label_2))
            (:3
              (goto _label))
            (:4
              (CallFunction|GetHitPenalty (Variables|Default|GetArmHitPenalty) :!label _label_3))
            (:5
              (goto _label_2))
            (:6
              (goto _label_3))
            (:7
              (goto _label_3))
            (:8
              (goto _label_2))
            (:9
              (goto _label_3))
            (:10
              (bind _reward (CallFunction|GetGlovePoints MyComp OtherComp :!label _label_4))
              (CallFunction|GetHitPenalty _reward))
            (:11
              (CallFunction|GetHitPenalty (Variables|Default|GethipHitPenalty)))
            (:12
              (goto _label_4))
            (:13
              (CallFunction|GetHitPenalty (Variables|Default|GetlegHitPenalty) :!label _label_5))
            (:14
              (goto _label_5))
            (:15
              (goto _label_5))
            (:16
              (goto _label_5))
            (:17
              (bind _reward_2 (CallFunction|SteppingReward _array_element :!label _label_6))
              (CallFunction|GetHitPenalty _reward_2))
            (:18
              (goto _label_6))))))))

(fn ConstructionScript)

(fn GetPhysicsInputs
  ;[0.1556 0.142 1] collect enemydata
  (bind _outactors (Actor|GetAllActorsOfClass "BP_Boxer_C"))
  (bind _array_element (Utilities|Array|ForEachLoopwithBreak _outactors :!label _label)
    (:LoopBody
      (if (!= _array_element self)
        (bind _output_get (LocalVariables|Setopponent _array_element))
        (goto _label Break)))
    (:Completed
      (for _index (range 0 18)
        ;[1 1 1] assign enemy Head instead of LeftForeArm
        (switch int _index
          (:Default
            ;[1 1 1] assign enemy middletorso instead of RightForeArm
            (switch int _index
              (:Default
                ;[1 1 1] Assign bodyparts as default
                (for _array_element_2 (Actor|GetComponentsbyTag "/Script/Engine.SceneComponent" (Utilities|String|StringToName (Utilities|String|ToString(Integer) _index)))
                  (Class|Boxer|SetVelocity _index (Transformation|GetComponentVelocity _array_element_2))
                  (Class|Boxer|SetPosition _index (Transformation|GetWorldLocation _array_element_2))))
              (:9
                (for _array_element_3 (Actor|GetComponentsbyTag _output_get "/Script/Engine.SceneComponent" "5")
                  (Class|Boxer|SetVelocity _index (Transformation|GetComponentVelocity _array_element_3))
                  (Class|Boxer|SetPosition _index (Transformation|GetWorldLocation _array_element_3))))))
          (:7
            (for _array_element_4 (Actor|GetComponentsbyTag _output_get "/Script/Engine.SceneComponent" "0")
              (Class|Boxer|SetVelocity _index (Transformation|GetComponentVelocity _array_element_4))
              (Class|Boxer|SetPosition _index (Transformation|GetWorldLocation _array_element_4)))))))))

(fn ApplyNeuralNetworkOutputs
  (for _index (range 0 18)
    (for _array_element (Actor|GetComponentsbyTag "/Script/Engine.PrimitiveComponent" (Utilities|String|StringToName (Utilities|String|ToString(Integer) _index)))
      (bind _returnvalue (Class|Boxer|GetForce _index))
      (Physics|AddForce _array_element _returnvalue "None" false))))

(fn TemplateFunciton)

(fn GetHitPenalty
  (params (regionHitPenalty :type Float%20%28single-precision%29))
  (if (not (Variables|Default|GethasStruckOpponent))
    (Variables|Default|SetHitScore (+ (Variables|Default|GetHitScore) regionHitPenalty))))

(fn GetFeetDistance
  (params (FeetTag :type Name))
  (for _array_element (Actor|GetComponentsbyTag "/Script/Engine.PrimitiveComponent" FeetTag)
    (return (Math|Vector2D|Vector2DLength (Math|Vector2D|MakeVector2D (.X (Math|Vector|BreakVector (Transformation|GetWorldLocation _array_element))) (.Y (Math|Vector|BreakVector (Transformation|GetWorldLocation _array_element))))))))

(fn SteppingReward
  (params (FeetTag :type Name))
  (bind _distance (CallFunction|GetFeetDistance FeetTag))
  (return (* (/ (LocalVariables|GetRewardScaling) (Math|Float|Square _distance)) (Variables|Default|GetFeetHitReward))))

(fn GetGlovePoints
  (params (glove :type Scene%20Component%20Object%20Reference) (targetHit :type Actor%20Component%20Object%20Reference))
  (if (Variables|Default|GethasStruckOpponent)
    (return (* (+ (Math|Vector|VectorLength (Transformation|GetComponentVelocity glove)) 1.0) (Variables|Default|GetGloveHitReward)))
    (else
      (return (Variables|Default|GetGloveHitPenalty)))))

(fn RewardProperStance
  (bind _outcomponents (Collision|BoxOverlapComponents "0.000000,0.000000,275.000000" "550.000000,550.000000,75.000000" (Utilities|Array|MakeArray "ObjectTypeQuery4") "/Script/Engine.StaticMeshComponent" 0 :!class /Script/Engine.KismetSystemLibrary))
  (for _array_element _outcomponents
    (for _array_element_2 (Variables|/Script/Engine.ActorComponent|GetComponentTags _array_element)
      (Variables|Default|SetOverlapScore (+ (Variables|Default|GetOverlapScore) (* (Variables|Default|GetProperStanceReward) (Math|Conversions|ToFloat(Boolean) (and (Utilities|Name|Equal(Name) _array_element_2 (Utilities|Name|MakeLiteralName "0")) (== (Components|GetOwner _array_element) self)))))))))